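; Cloud actor that spawns a set of CloudParticle actors at BeginPlay, attaches them to its root and passes them its spawn volume.
; Custom events forward color, intensity and scale limits to the particles and resize the spawn sphere.
; Holding F starts damage trails and a camera shake; releasing it ends the trails after a short delay.
; No damage is applied here: the TakeDamage timer is only cleared, never set.
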(event Custom|StartDamaging
  (if (not (Variables|Default|GetIsDamaging))
    (Effects|Particles|Trails|BeginTrails (Variables|Default|GetDamageParticle) "None" "None" "ETrailWidthMode_FromCentre" 0.0)
    (Variables|Default|SetIsDamaging true)
    (Camera|PlayWorldCameraShake "/Script/Engine.CameraShake" "0.000000, 0, 0" 1e+02 1e+03 1e+03)))

(event Custom|UpdateCloud
  (Components|Sphere|SetSphereRadius (Variables|Default|GetParticleSpawn) (Variables|Default|GetSpawnRadius) true))

(event Custom|StopDamaging
  (if (Variables|Default|GetIsDamaging)
    (Variables|Default|SetIsDamaging false)
    (Utilities|Time|ClearTimerbyFunctionName 0 "TakeDamage")
    (Utilities|FlowControl|Delay 0.8)
    (if (not (Variables|Default|GetIsDamaging))
      (Effects|Particles|Trails|EndTrails (Variables|Default|GetDamageParticle)))))

(event Custom|UpdateParticles
  (for _array_element (Variables|Default|GetParticles)
    (Variables|/Game/Blueprints/CloudParticle.CloudParticle_C|SetMinScale _array_element (Variables|Default|GetMinParticleScale))
    (Variables|/Game/Blueprints/CloudParticle.CloudParticle_C|SetMaxScale _array_element (Variables|Default|GetMaxParticleScale))))

(event Custom|SetParticleColor
  (params (Color :type Linear%20Color%20Structure))
  (for _array_element (Variables|Default|GetParticles)
    (Default|SetColor _array_element Color)))

(event Custom|SetIntensity
  (params (Intensity :type Float%20%28single-precision%29))
  (for _array_element (Variables|Default|GetParticles)
    (Default|SetIntensity _array_element Intensity)))

(event EventBeginPlay
  (Utilities|FlowControl|Sequence
    (:then_0
      (Input|EnableInput (Game|GetPlayerController 0))
      (CallFunction|StopDamaging))
    (:then_1
      (for _index (range 1 (Variables|Default|GetParticleCount))
        (bind _returnvalue (Game|SpawnActorfromClass "/Game/Blueprints/CloudParticle.CloudParticle_C" (Transformation|GetWorldTransform (Variables|Default|GetDefaultSceneRoot)) "Undefined" 0 0))
        (Variables|/Game/Blueprints/CloudParticle.CloudParticle_C|SetParticleSpawn _returnvalue (Variables|Default|GetParticleSpawn))
        (Transformation|AttachComponentToComponent _returnvalue (Variables|Default|GetDefaultSceneRoot) "None" "SnapToTarget" "SnapToTarget" "KeepWorld" true)
        (Utilities|Array|Add (Variables|Default|GetParticles) _returnvalue)))
    (:then_2
      (Effects|Particles|Trails|EndTrails (Variables|Default|GetDamageParticle)))))

(event Input|KeyboardEvents|F
  (params (Key :type Key%20Structure :default "AnyKey"))
  (:Pressed
    (CallFunction|StartDamaging))
  (:Released
    (CallFunction|StopDamaging)))

(fn ConstructionScript)