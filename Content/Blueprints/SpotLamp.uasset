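; SpotLamp is a lamp actor that hurts the player inside its trigger until it is charged past a threshold.
; Gaze focus, the L key or nearby Interact raises a clamped Ratio each tick, which decays when released.
; Ratio drives cone angle, trigger radius and light color.
; Threshold crossings toggle damage and wall collision, though the wall only returns if the player is overlapping; BeginPlay also attaches spawned CrazySpotLights.
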(event Custom|StartShining
  (if (not (Variables|Default|GetIsIncreasing))
    (Variables|Default|SetIsIncreasing true)))

(event Custom|StartDamaging
  (bind _asmain_player_character (Utilities|Casting|CastToMainPlayerCharacter (Game|Player|GetPlayerPawn 0)))
  (Default|StartDamaging _asmain_player_character))

(event Custom|StopShining
  (if (Variables|Default|GetIsIncreasing)
    (Variables|Default|SetIsIncreasing false)))

(event Custom|UpdateThreshold
  (Utilities|FlowControl|Sequence
    (:then_0
      (if (and (< (Variables|Default|GetOldRatio) (Variables|Default|GetThreshold)) (>= (Variables|Default|GetRatio) (Variables|Default|GetThreshold)))
        (bind _returnvalue (Audio|SpawnSound2D (Variables|Default|GetEnableSound)))
        (Collision|SetCollisionEnabled (Variables|Default|GetWallCollision) "NoCollision")
        (Audio|Components|Audio|Play _returnvalue 0.0)
        (if (Variables|Default|GetIsCollidingPlayer)
          (CallFunction|StopDamaging))))
    (:then_1
      (if (and (and (>= (Variables|Default|GetOldRatio) (Variables|Default|GetThreshold)) (< (Variables|Default|GetRatio) (Variables|Default|GetThreshold))) (Variables|Default|GetIsCollidingPlayer))
        (CallFunction|StartDamaging)
        (Collision|SetCollisionEnabled (Variables|Default|GetWallCollision) "QueryAndPhysics")))))

(event Custom|StopDamaging
  (bind _asmain_player_character (Utilities|Casting|CastToMainPlayerCharacter (Game|Player|GetPlayerPawn 0)))
  (Default|StopDamaging _asmain_player_character))

(event Custom|UpdateFromRatio
  (bind _ratio (Variables|Default|GetRatio))
  (bind _minspotradius (Variables|Default|GetMinSpotRadius))
  (bind _maxspotradius (Variables|Default|GetMaxSpotRadius))
  (bind _spotlight (Variables|Default|GetSpotLight))
  (bind _fromcolor (Variables|Default|GetFromColor))
  (bind _tocolor (Variables|Default|GetToColor))
  (bind _returnvalue (Math|Float|MapRangeClamped _ratio 0.0 1.0 _minspotradius _maxspotradius))
  (bind _returnvalue_2 (Math|Color|Lerp(LinearColor) _fromcolor _tocolor _ratio))
  (Rendering|Lighting|SetOuterConeAngle _spotlight _returnvalue)
  (Rendering|Lighting|SetInnerConeAngle _spotlight (/ _returnvalue 1.2))
  (Components|Capsule|SetCapsuleRadius (Variables|Default|GetTriggerCapsule) (Math|Float|MapRangeClamped _ratio 0.0 1.0 (Variables|Default|GetMinTriggerRadius) (Variables|Default|GetMaxTriggerRadius)) true)
  (Rendering|Components|Light|SetLightColor (Variables|Default|GetSpotLight) _returnvalue_2 true)
  (Rendering|Components|Light|SetLightColor (Variables|Default|GetPointLight) _returnvalue_2 true)
  (Variables|Default|SetIsEnabled (>= (Variables|Default|GetRatio) (Variables|Default|GetThreshold)))
  (CallFunction|UpdateThreshold))

(event EventBeginPlay
  (Utilities|FlowControl|Sequence
    (:then_0
      (Input|EnableInput (Game|GetPlayerController 0)))
    (:then_1
      (for _index (range 1 (Variables|Default|GetSpotLightCount))
        (bind _returnvalue (Game|SpawnActorfromClass "/Game/Blueprints/CrazySpotLight.CrazySpotLight_C" (Transformation|GetWorldTransform (Variables|Default|GetDefaultSceneRoot)) "Undefined" 0 0))
        (Transformation|AttachComponentToComponent _returnvalue (Variables|Default|GetDefaultSceneRoot) "None" "SnapToTarget" "SnapToTarget" "KeepWorld" true)))))

(event EventLostGazeFocusBP
  (CallFunction|StopShining))

(event Collision|EventActorBeginOverlap
  (params (OtherActor :type Actor%20Object%20Reference))
  (Utilities|Casting|CastToMainPlayerCharacter OtherActor)
  (Variables|Default|SetIsCollidingPlayer true)
  (if (not (Variables|Default|GetIsEnabled))
    (CallFunction|StartDamaging)))

(event Collision|EventActorEndOverlap
  (params (OtherActor :type Actor%20Object%20Reference))
  (Utilities|Casting|CastToMainPlayerCharacter OtherActor)
  (Variables|Default|SetIsCollidingPlayer false)
  (CallFunction|StopDamaging))

(event EventTick
  (params (DeltaSeconds :type Float%20%28single-precision%29))
  (Variables|Default|SetOldRatio (Variables|Default|GetRatio))
  (Variables|Default|SetRatio (Math|Float|Clamp(Float) (+ (* DeltaSeconds (select (Variables|Default|GetIsIncreasing) (Variables|Default|GetIncreaseSpeed) (* (Variables|Default|GetDecreaseSpeed) -1.0))) (Variables|Default|GetRatio))))
  (CallFunction|UpdatefromRatio))

(event EventGotGazeFocusBP
  (CallFunction|StartShining))

(event Input|ActionEvents|InputActionInteract
  (params (Key :type Key%20Structure :default "AnyKey"))
  (:Pressed
    (if (<= (Math|Vector|VectorLength (- (Transformation|GetActorLocation (Game|Player|GetPlayerPawn 0)) (Transformation|GetWorldLocation (Variables|Default|GetDefaultSceneRoot)))) (Variables|Default|GetInteractionDistance))
      (CallFunction|StartShining)))
  (:Released
    (CallFunction|StopShining)))

(event Input|KeyboardEvents|L
  (params (Key :type Key%20Structure :default "AnyKey"))
  (:Pressed
    (CallFunction|StartShining))
  (:Released
    (CallFunction|StopShining)))

(fn ConstructionScript)