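; FollowTrajectoryMovement moves the player along a trajectory's hit points in light mode, with looping controller vibration.
; FollowTrajectory freezes trajectory updates, prepends the trajectory actor's location, hides it and builds a temporary spline from the points.
; The pawn travels the spline in a time derived from length and Speed.
; Timed delays then resume trajectory updates and, shortly after, end light mode and vibration.
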(event Custom|FollowTrajectory
  (params (Trajetory :type Reflection%20Trajectory%20Object%20Reference))
  (bind _hitlocations (Variables|/Game/Blueprints/ReflectionTrajectory.ReflectionTrajectory_C|GetHitLocations Trajetory))
  (bind _asmain_player_character (Utilities|Casting|CastToMainPlayerCharacter (Game|Player|GetPlayerPawn 0)))
  (Default|StartLightMode _asmain_player_character)
  (Game|Feedback|ClientPlayForceFeedback (Game|GetPlayerController 0) "/Game/Blueprints/LightReflectionVibration.LightReflectionVibration" true "None")
  (Variables|/Game/Blueprints/ReflectionTrajectory.ReflectionTrajectory_C|SetAutoUpdate Trajetory false)
  (Utilities|Array|Insert _hitlocations (Transformation|GetActorLocation (Components|GetOwner (Variables|/Game/Blueprints/ReflectionTrajectory.ReflectionTrajectory_C|GetDefaultSceneRoot Trajetory))))
  (if (> (Utilities|Array|Length _hitlocations) 0)
    (Rendering|SetVisibility (Variables|/Game/Blueprints/ReflectionTrajectory.ReflectionTrajectory_C|GetDefaultSceneRoot Trajetory) false true)
    (bind _splinecomponent (Class|ITween|GenerateSplinefromVectorArray "0, 0, 0" "0, 0, 0" _hitlocations false false))
    (Class|ITween|ActorMovetoSplinePointSimple "No Name" (Game|Player|GetPlayerPawn 0) _splinecomponent false false (* (Spline|GetSplineLength _splinecomponent) (/ 1.0 (Variables|Default|GetSpeed))) "linear" "" 0 0 0 0 true)
    (Utilities|FlowControl|Delay (* (Spline|GetSplineLength _splinecomponent) (/ 1.0 (Variables|Default|GetSpeed))))
    (Variables|/Game/Blueprints/ReflectionTrajectory.ReflectionTrajectory_C|SetAutoUpdate Trajetory true)
    (Utilities|FlowControl|Delay 0.75)
    (Default|StopLightMode _asmain_player_character)
    (Game|Feedback|ClientStopForceFeedback (Game|GetPlayerController 0) "/Game/Blueprints/LightReflectionVibration.LightReflectionVibration" "None")))