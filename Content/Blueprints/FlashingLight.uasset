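; FlashingLight is a Blueprint that continuously animates the intensity and color of a point light.
; A looping Animation timeline starts on BeginPlay and replays from the start whenever it finishes.
; Its Color track maps to the Min/Max intensity range scaled by IntensityMultiplier, while its Intensity track blends MinColor to MaxColor, so the track names are crossed relative to their use.
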(event EventBeginPlay
  (bind _pointlight (Variables|Default|GetPointLight))
  (bind (_direction _color _intensity) (Timeline|Animation Play)
    (:Update
      (Rendering|Components|Light|SetIntensity _pointlight (* (Math|Float|MapRangeClamped _color 0.0 1.0 (Variables|Default|GetMinIntensity) (Variables|Default|GetMaxIntensity)) (Variables|Default|GetIntensityMultiplier)))
      (Rendering|Components|Light|SetLightColor _pointlight (Math|Color|Lerp(LinearColor) (Variables|Default|GetMinColor) (Variables|Default|GetMaxColor) _intensity) true))
    (:Finished
      (Timeline|Animation PlayFromStart))))

(fn ConstructionScript)