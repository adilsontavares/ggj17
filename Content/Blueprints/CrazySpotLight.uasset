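; CrazySpotLight is an actor, named as a spotlight, that endlessly swings to random orientations.
; After a random startup delay, a self-calling event tweens the actor from its current rotation toward a random direction vector using ActorRotateFromToSimple.
; Each cycle then waits a random rotation time plus a random sleep before repeating.
; That wait rolls its rotation time separately from the tween, so the two durations can differ.
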(event Custom|RotateToRandomRotator
  (bind _minrotateduration (Variables|Default|GetMinRotateDuration))
  (bind _maxrotateduration (Variables|Default|GetMaxRotateDuration))
  (bind _returnvalue (Math|Random|RandomFloatinRange _minrotateduration _maxrotateduration))
  (Class|ITween|ActorRotatefromtoSimple "No Name" self (Transformation|GetWorldRotation (Variables|Default|GetDefaultSceneRoot)) (Math|Conversions|RotationFromXVector (Math|Vector|MakeVector (Math|Random|RandomFloatinRange -1.0 1.0) (Math|Random|RandomFloatinRange -1.0 1.0) (Math|Random|RandomFloatinRange -1.0 1.0))) "world" false _returnvalue "linear")
  (Utilities|FlowControl|Delay (+ _returnvalue (Math|Random|RandomFloatinRange (Variables|Default|GetMinSleep) (Variables|Default|GetMaxSleep))))
  (CallFunction|RotatetoRandomRotator))

(event EventBeginPlay
  (Utilities|FlowControl|Delay (Math|Random|RandomFloatinRange (Variables|Default|GetMinSleep) (Variables|Default|GetMaxSleep)))
  (CallFunction|RotatetoRandomRotator))

(fn ConstructionScript)