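; Actor that predicts a ray's bouncing path off surfaces tagged Reflectable, optionally updating every tick from its root's transform.
; A recursive line trace stores each impact and mirrors the direction by the hit normal, up to PredictionCount bounces.
; When a trace misses or hits a non-reflectable actor, it draws randomly colored debug lines from the player pawn through the stored points if visible.
; The arrow-marker logic is disconnected.
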(event Custom|UpdateTrajetory
  (params (RayPosition :type Vector) (RayDirection :type Vector) (StartIndex :type Integer))
  ;[1 1 1] Update trajetory
  (if (== StartIndex 0)
    (Utilities|Array|Clear (Variables|Default|GetHitLocations)))
  (if (< StartIndex (Variables|Default|GetPredictionCount))
    (bind (_outhit _returnvalue) (Collision|LineTraceByChannel RayPosition (+ RayPosition (* RayDirection 1e+03)) "TraceTypeQuery1" false 0 "None"))
    (if _returnvalue
      (if (Actor|ActorHasTag (.HitActor (Collision|BreakHitResult _outhit)) "Reflectable")
        (Utilities|Array|Add (Variables|Default|GetHitLocations) (.ImpactPoint (Collision|BreakHitResult _outhit)))
        (CallFunction|UpdateTrajetory (+ (.ImpactPoint (Collision|BreakHitResult _outhit)) (.Normal (Collision|BreakHitResult _outhit))) (Math|Vector|Normalize (Math|Vector|MirrorVectorbyNormal (- (.TraceEnd (Collision|BreakHitResult _outhit)) (.TraceStart (Collision|BreakHitResult _outhit))) (.Normal (Collision|BreakHitResult _outhit)))) (+ StartIndex 1))
        (else
          (CallFunction|HidefromIndex StartIndex :!label _label)
          ;[1 1 1] Print line debug
          (if (Rendering|IsVisible (Variables|Default|GetDefaultSceneRoot))
            (for (_array_element _array_index) (Variables|Default|GetHitLocations)
              (CallFunction|DrawDebugLine (select (== _array_index 0) (Transformation|GetActorLocation (Game|Player|GetPlayerPawn 0)) (Utilities|Array|Get(acopy) (Variables|Default|GetHitLocations) (- _array_index 1))) _array_element)))))
      (else
        (goto _label)))
    (else
      (CallFunction|HidefromIndex StartIndex))))

(event Custom|HideFromIndex
  (params (Index :type Integer))
  ;[1 1 1] Hide unwanted arrows
)

(event Custom|DrawDebugLine
  (params (FromLocation :type Vector) (ToLocation :type Vector))
  (bind _returnvalue (Math|Random|RandomFloatinRange 0.0 1.0))
  ;[1 1 1] Draws debug line
  (Rendering|Debug|DrawDebugLine FromLocation ToLocation (Math|Color|MakeColor _returnvalue _returnvalue _returnvalue) 0.1 0.0))

(event Custom|UpdateTrajetoryFromTransform
  (bind _defaultsceneroot (Variables|Default|GetDefaultSceneRoot))
  ;[1 1 1] Update from transform
  (CallFunction|UpdateTrajetory (Transformation|GetWorldLocation _defaultsceneroot) (Math|Rotator|GetRotationXVector (Transformation|GetWorldRotation _defaultsceneroot))))

(event EventBeginPlay
  (Input|EnableInput (Game|GetPlayerController 0)))

(event EventTick
  (params (DeltaSeconds :type Float%20%28single-precision%29))
  ;[1 1 1] Main loop
  (if (Variables|Default|GetAutoUpdate)
    (CallFunction|UpdateTrajetoryfromTransform)))

(fn ConstructionScript)