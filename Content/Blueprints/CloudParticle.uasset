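; Cloud particle actor that drifts around a spawn sphere while pulsing in size, with externally settable material color and intensity.
; A recursive event tweens it to random offsets within radius-sized bounds around ParticleSpawn, then waits a separately randomized duration before repeating.
; Tick uses a DoOnce, reset when the UpdateScale timeline finishes, to replay that timeline, mapping its curve uniformly between minimum and maximum scale.
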(event Custom|MoveParticleToRandomPosition
  (bind _minmoveduration (Variables|Default|GetMinMoveDuration))
  (bind _maxmoveduration (Variables|Default|GetMaxMoveDuration))
  (bind _particlespawn (Variables|Default|GetParticleSpawn))
  (bind _returnvalue (Math|Random|RandomFloatinRange _minmoveduration _maxmoveduration))
  (bind _sphereradius (Variables|/Script/Engine.SphereComponent|GetSphereRadius _particlespawn))
  (bind _returnvalue_2 (* _sphereradius -1.0))
  (Class|ITween|ActorMovefromtoSimple "MoveParticle" self (Transformation|GetWorldLocation (Variables|Default|GetScene)) (+ (Transformation|GetWorldLocation _particlespawn) (Math|Vector|MakeVector (Math|Random|RandomFloatinRange _returnvalue_2 _sphereradius) (Math|Random|RandomFloatinRange _returnvalue_2 _sphereradius) (Math|Random|RandomFloatinRange _returnvalue_2 _sphereradius))) "world" false _returnvalue "linear")
  (Utilities|FlowControl|Delay _returnvalue)
  (CallFunction|MoveParticletoRandomPosition))

(event Custom|SetColor
  (params (Color :type Linear%20Color%20Structure))
  (bind (_r _g _b) (Utilities|Struct|BreakLinearColor Color))
  ;[1 1 1] Update material color
  (Rendering|Material|SetVectorParameterValueonMaterials (Variables|Default|GetSphere) "Color" (Math|Vector|MakeVector _r _g _b)))

(event Custom|SetIntensity
  (params (Intensity :type Float%20%28single-precision%29))
  ;[1 1 1] Update material intensity
  (Rendering|Material|SetScalarParameterValueonMaterials (Variables|Default|GetSphere) "Intensity" Intensity))

(event EventTick
  (params (DeltaSeconds :type Float%20%28single-precision%29))
  (Utilities|FlowControl|DoOnce true :!label _label
    (:Completed
      (bind _scale (Timeline|UpdateScale PlayFromStart)
        (:Update
          (Transformation|SetWorldScale3D (Variables|Default|GetScene) (Math|Vector|MakeVector (Math|Float|MapRangeClamped _scale 0.0 1.0 (Variables|Default|GetMinScale) (Variables|Default|GetMaxScale)) (Math|Float|MapRangeClamped _scale 0.0 1.0 (Variables|Default|GetMinScale) (Variables|Default|GetMaxScale)) (Math|Float|MapRangeClamped _scale 0.0 1.0 (Variables|Default|GetMinScale) (Variables|Default|GetMaxScale)))))
        (:Finished
          (goto _label Reset))))))

(event EventBeginPlay
  (Utilities|FlowControl|Sequence
    (:then_0
      (bind _scale (Timeline|UpdateScale SetNewTime)
        (:Update
          (Transformation|SetWorldScale3D (Variables|Default|GetScene) (Math|Vector|MakeVector (Math|Float|MapRangeClamped _scale 0.0 1.0 (Variables|Default|GetMinScale) (Variables|Default|GetMaxScale)) (Math|Float|MapRangeClamped _scale 0.0 1.0 (Variables|Default|GetMinScale) (Variables|Default|GetMaxScale)) (Math|Float|MapRangeClamped _scale 0.0 1.0 (Variables|Default|GetMinScale) (Variables|Default|GetMaxScale)))))
        (:Finished
          (Utilities|FlowControl|DoOnce true) ; enters at Reset
        )))
    (:then_1
      (Timeline|UpdateScale Play))
    (:then_2
      (CallFunction|MoveParticletoRandomPosition))))

(fn ConstructionScript)