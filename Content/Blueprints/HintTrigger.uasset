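; HintTrigger is a trigger actor that shows a button hint on the HUD while the player character overlaps it.
; On begin overlap with MainPlayerCharacter, it gets MainHUD from player controller 0 and passes its InputType variable to the ButtonHint widget's ShowHint.
; On end overlap, it runs the same character and HUD casts, then calls HideHint.
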(event Collision|EventActorBeginOverlap
  (params (OtherActor :type Actor%20Object%20Reference))
  (Utilities|Casting|CastToMainPlayerCharacter OtherActor)
  (bind _asmain_hud (Utilities|Casting|CastToMainHUD (HUD|GetHUD (Game|GetPlayerController 0))))
  (Default|ShowHint (Variables|/Game/Blueprints/MainHUD.MainHUD_C|GetButtonHint _asmain_hud) (Variables|Default|GetInputType)))

(event Collision|EventActorEndOverlap
  (params (OtherActor :type Actor%20Object%20Reference))
  (Utilities|Casting|CastToMainPlayerCharacter OtherActor)
  (Utilities|Casting|CastToMainHUD (HUD|GetHUD (Game|GetPlayerController 0)))
  (Default|HideHint (Variables|/Game/Blueprints/MainHUD.MainHUD_C|GetButtonHint (stale Collision|EventActorBeginOverlap _asmain_hud))))

(fn ConstructionScript)