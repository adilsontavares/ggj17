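; Checkpoint actor that refills the player's health when the main character overlaps it, then goes dark.
; Consume disables its box collision and pawn input, plays camera shake, sound and controller vibration, and starts a timeline lerping Health to full.
; After a delay it swaps to the broken mesh, hides the point light and restores input.
; The H key also fires Consume directly, bypassing the overlap.
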(event Custom|Break
  ;[1 1 1] Break light
  (Rendering|SetVisibility (Variables|Default|GetMeshBefore) false false)
  (Rendering|SetVisibility (Variables|Default|GetMeshAfter) true false)
  (Rendering|SetVisibility (Variables|Default|GetPointLight) false false))

(event Custom|Consume
  ;[1 1 1] Consume light
  (Class|PlayerCameraManager|PlayCameraShake (Game|GetPlayerCameraManager 0) "/Game/Blueprints/CheckpointCameraShake.CheckpointCameraShake_C" 1.0 "World" "0, 0, 0")
  (Input|DisableInput (Game|Player|GetPlayerPawn 0) 0)
  (CallFunction|RechargePlayer)
  (Collision|SetCollisionEnabled (Variables|Default|GetBox) "NoCollision")
  (bind _returnvalue (Audio|CreateSound2D "/Game/Audio/Choque_com_Reverb.Choque_com_Reverb"))
  (Audio|Components|Audio|Play _returnvalue 0.0)
  (Audio|Components|Audio|FadeIn _returnvalue 0.6 1.0 0.0 :!class /Script/Engine.AudioComponent)
  (Game|Feedback|ClientPlayForceFeedback (Game|GetPlayerController 0) "/Game/Blueprints/CheckpointVibration.CheckpointVibration" false "None")
  (Utilities|FlowControl|Delay 2.8)
  (bind _returnvalue_2 (Audio|CreateSound2D "/Game/Audio/Check_Point.Check_Point"))
  (Audio|Components|Audio|Play _returnvalue_2 1.0)
  (CallFunction|Break)
  (Audio|Components|Audio|FadeOut _returnvalue 0.6 0.0 :!class /Script/Engine.AudioComponent)
  (Input|EnableInput (Game|Player|GetPlayerPawn 0) 0))

(event Custom|RechargePlayer
  ;[1 1 1] Recharge player
  (bind _asmain_player_character (Utilities|Casting|CastToMainPlayerCharacter (Game|GetPlayerCharacter 0)))
  (bind _output_get (Variables|Default|SetFromHealth (Variables|/Game/Blueprints/MainPlayerCharacter.MainPlayerCharacter_C|GetHealth _asmain_player_character)))
  (bind _alpha (Timeline|Regenerate PlayFromStart)
    (:Update
      (Variables|/Game/Blueprints/MainPlayerCharacter.MainPlayerCharacter_C|SetHealth _asmain_player_character (Math|Float|Lerp _output_get 1e+02 _alpha)))))

(event EventBeginPlay
  (Input|EnableInput (Game|GetPlayerController 0)))

(event Collision|EventActorBeginOverlap
  (params (OtherActor :type Actor%20Object%20Reference))
  (Utilities|Casting|CastToMainPlayerCharacter OtherActor)
  (CallFunction|Consume))

(event Input|KeyboardEvents|H
  (params (Key :type Key%20Structure :default "AnyKey"))
  (:Pressed
    (CallFunction|Consume)))

(fn ConstructionScript)