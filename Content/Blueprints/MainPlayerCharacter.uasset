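; Player character for side-on movement locked to Y=0, embodied as a particle cloud with a flashing light.
; BeginPlay attaches spawned Cloud, FlashingLight and stick-aimed ReflectionTrajectory actors; Tick updates zoom and scales the cloud by Health.
; Light dash follows trajectory hits or launches in a brief light mode that recolors and ignores a custom collision channel; particle dash just launches.
; "Damagable" overlaps toggle damage effects without changing Health, which only debug keys alter.
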(event Custom|StartDamaging
  ;[1 1 1] Damages
  (if (not (Variables|Default|GetIsDamaging))
    (Variables|Default|SetIsDamaging true)
    (Game|Feedback|ClientPlayForceFeedback (Game|GetPlayerController 0) "/Game/Blueprints/DamageVibration.DamageVibration" true "DamageVibration")
    (Default|StartDamaging (Variables|Default|GetCloud))
    (bind _returnvalue (Audio|SpawnSound2D "/Game/Audio/Choque_com_Reverb.Choque_com_Reverb"))
    (Audio|Components|Audio|FadeIn _returnvalue 0.5 1.0 0.0 :!class /Script/Engine.AudioComponent)))

(event Custom|UpdateReflectionTrajetory
  (bind _returnvalue (Input|AxisValues|GetLookRight))
  (bind _returnvalue_2 (Input|AxisValues|GetLookUp))
  (bind _reflectiontrajectory (Variables|Default|GetReflectionTrajectory))
  (bind _returnvalue_3 (Math|Vector|MakeVector _returnvalue 0.0 _returnvalue_2))
  (bind _defaultsceneroot (Variables|/Game/Blueprints/ReflectionTrajectory.ReflectionTrajectory_C|GetDefaultSceneRoot _reflectiontrajectory))
  ;[1 1 1] Update reflection trajetory
  (Rendering|SetVisibility _defaultsceneroot (>= (Math|Vector|VectorLength _returnvalue_3) 0.1) false)
  (if true
    (Transformation|SetWorldRotation _defaultsceneroot (Math|Rotator|MakeRotfromX _returnvalue_3) false false)))

(event Custom|UpdateHealth
  (bind _health (Variables|Default|GetHealth))
  (bind _cloud (Variables|Default|GetCloud))
  (bind _returnvalue (Math|Float|MapRangeUnclamped _health 0.0 1e+02 0.2 5.0))
  ;[1 1 1] Update player health
  (Default|SetIntensity (Variables|Default|GetCloud) (select (Variables|Default|GetIsLight) (* _returnvalue 5.0) _returnvalue))
  (Variables|/Game/Blueprints/Cloud.Cloud_C|SetMinParticleScale _cloud (Math|Float|MapRangeClamped _health 0.0 1e+02 0.06 0.6))
  (Variables|/Game/Blueprints/Cloud.Cloud_C|SetMaxParticleScale _cloud (Math|Float|MapRangeClamped _health 0.0 1e+02 0.2 1.0))
  (Default|UpdateParticles _cloud)
  (Variables|/Game/Blueprints/Cloud.Cloud_C|SetSpawnRadius _cloud (Math|Float|MapRangeClamped _health 0.0 1e+02 25.0 32.0))
  (Default|UpdateCloud _cloud))

(event Custom|PlayDashVibration
  (params (Force%20Feedback%20Effect :type Force%20Feedback%20Effect%20Object%20Reference))
  ;[1 1 1] Dash vibration
  (Game|Feedback|ClientPlayForceFeedback (Game|GetPlayerController 0) Force%20Feedback%20Effect false "None"))

(event Custom|StartLightMode
  (bind _flashinglight (Variables|Default|GetFlashingLight))
  ;[1 1 1] Handle light mode
  (if (not (Variables|Default|GetIsLight))
    (Variables|Default|SetIsLight true)
    (Utilities|FlowControl|Sequence
      (:then_0
        (Collision|SetCollisionResponsetoChannel (Variables|Collision|GetCapsuleComponent) "ECC_GameTraceChannel1" "ECR_Ignore"))
      (:then_1
        (Default|SetIntensity (Variables|Default|GetCloud) 3e+01)
        (bind _output_get (Variables|Default|SetColor (Variables|Default|GetLightColor)))
        (Variables|/Game/Blueprints/FlashingLight.FlashingLight_C|SetMinColor _flashinglight (Utilities|Struct|MakeLinearColor (* (.R (Utilities|Struct|BreakLinearColor _output_get)) 0.5) (* (.G (Utilities|Struct|BreakLinearColor _output_get)) 0.5) (* (.B (Utilities|Struct|BreakLinearColor _output_get)) 0.5) (.A (Utilities|Struct|BreakLinearColor _output_get))))
        (Variables|/Game/Blueprints/FlashingLight.FlashingLight_C|SetMaxColor _flashinglight (Utilities|Struct|MakeLinearColor (* (.R (Utilities|Struct|BreakLinearColor (Variables|Default|GetColor))) 1.3) (* (.G (Utilities|Struct|BreakLinearColor (Variables|Default|GetColor))) 1.3) (* (.B (Utilities|Struct|BreakLinearColor (Variables|Default|GetColor))) 1.3) (.A (Utilities|Struct|BreakLinearColor (Variables|Default|GetColor)))))
        (Default|SetParticleColor (Variables|Default|GetCloud) (Variables|Default|GetColor))))))

(event Custom|StopLightMode
  (bind _flashinglight (Variables|Default|GetFlashingLight))
  ;[1 1 1] Handle light mode
  (if (Variables|Default|GetIsLight)
    (Variables|Default|SetIsLight false)
    (Default|SetIntensity (Variables|Default|GetCloud) 4.0)
    (Utilities|FlowControl|Sequence
      (:then_0
        (Variables|Default|SetColor (Variables|Default|GetParticleColor))
        (Variables|/Game/Blueprints/FlashingLight.FlashingLight_C|SetMinColor _flashinglight (Utilities|Struct|MakeLinearColor (* (.R (Utilities|Struct|BreakLinearColor (stale Custom|StartLightMode _output_get))) 0.5) (* (.G (Utilities|Struct|BreakLinearColor (stale Custom|StartLightMode _output_get))) 0.5) (* (.B (Utilities|Struct|BreakLinearColor (stale Custom|StartLightMode _output_get))) 0.5) (.A (Utilities|Struct|BreakLinearColor (stale Custom|StartLightMode _output_get)))))
        (Variables|/Game/Blueprints/FlashingLight.FlashingLight_C|SetMaxColor _flashinglight (Utilities|Struct|MakeLinearColor (* (.R (Utilities|Struct|BreakLinearColor (Variables|Default|GetColor))) 1.3) (* (.G (Utilities|Struct|BreakLinearColor (Variables|Default|GetColor))) 1.3) (* (.B (Utilities|Struct|BreakLinearColor (Variables|Default|GetColor))) 1.3) (.A (Utilities|Struct|BreakLinearColor (Variables|Default|GetColor)))))
        (Default|SetParticleColor (Variables|Default|GetCloud) (Variables|Default|GetColor)))
      (:then_1
        (Collision|SetCollisionResponsetoChannel (Variables|Collision|GetCapsuleComponent) "ECC_GameTraceChannel1" "ECR_Block")))))

(event Custom|StopDamaging
  ;[1 1 1] Damages
  (if (Variables|Default|GetIsDamaging)
    (Variables|Default|SetIsDamaging false)
    (Game|Feedback|ClientStopForceFeedback (Game|GetPlayerController 0) 0 "DamageVibration")
    (Default|StopDamaging (Variables|Default|GetCloud))
    (Utilities|FlowControl|Delay 0.7)
    (Audio|Components|Audio|FadeOut (stale Custom|StartDamaging _returnvalue) 1.0 0.0 :!class /Script/Engine.AudioComponent)
    (Components|DestroyComponent (stale Custom|StartDamaging _returnvalue))))

(event Custom|UpdateReflectionTrajectoryMouse
  (bind _returnvalue (Game|GetPlayerController 0))
  (bind (_locationx _locationy) (Game|Player|GetMousePosition _returnvalue))
  (bind _returnvalue_2 (Class|PlayerController|GetFocalLocation _returnvalue))
  (bind _returnvalue_3 (Math|Vector2D|MakeVector2D _locationx _locationy))
  (bind _screenposition (Class|GameplayStatics|ProjectWorldtoScreen _returnvalue _returnvalue_2 false))
  (bind _returnvalue_4 (- _screenposition _returnvalue_3))
  (bind (_x _y) (Math|Vector2D|BreakVector2D _returnvalue_4))
  ;[1 1 1] Update Reflection Trajectory Mouse
  (Transformation|SetWorldRotation (Variables|/Game/Blueprints/ReflectionTrajectory.ReflectionTrajectory_C|GetDefaultSceneRoot (Variables|Default|GetReflectionTrajectory)) (Math|Rotator|MakeRotfromX (Math|Vector|MakeVector (* _x -1.0) 0.0 _y)) false false))

(event Custom|UpdateZoom
  (bind _returnvalue (Input|AxisValues|GetZoomIn))
  (bind _returnvalue_2 (Input|AxisValues|GetZoomOut))
  (bind _zoominamount (Variables|Default|GetZoomInAmount))
  (bind _zoomoutamount (Variables|Default|GetZoomOutAmount))
  (bind _returnvalue_3 (* _returnvalue _zoominamount -1.0))
  (bind _returnvalue_4 (* _returnvalue_2 _zoomoutamount))
  (bind _returnvalue_5 (+ _returnvalue_3 _returnvalue_4))
  ;[1 1 1] Update zoom
  (Variables|/Script/Engine.SpringArmComponent|SetTargetOffset (Variables|Default|GetSpringArm) (Math|Vector|MakeVector 0.0 _returnvalue_5 (Math|Float|Clamp(Float) (* _returnvalue_5 0.3) 0.0 9999999.0))))

(event EventBeginPlay
  (Utilities|FlowControl|Sequence
    (:then_0
      ;[1 1 1] Spawn reflection trajetory
      (bind _returnvalue (Game|SpawnActorfromClass "/Game/Blueprints/ReflectionTrajectory.ReflectionTrajectory_C" (Transformation|GetWorldTransform (Variables|Collision|GetCapsuleComponent)) "Undefined" 0 0))
      (Transformation|AttachComponentToComponent (Variables|/Game/Blueprints/ReflectionTrajectory.ReflectionTrajectory_C|GetDefaultSceneRoot _returnvalue) (Variables|Collision|GetCapsuleComponent) "None" "SnapToTarget" "SnapToTarget" "KeepWorld" true)
      (Variables|Default|SetReflectionTrajectory _returnvalue))
    (:then_1
      ;[1 1 1] Spawn Cloud
      (bind _returnvalue_2 (Game|SpawnActorfromClass "/Game/Blueprints/Cloud.Cloud_C" (Transformation|GetWorldTransform (Variables|Collision|GetCapsuleComponent)) "Undefined" 0 0))
      (bind _output_get (Variables|Default|SetCloud _returnvalue_2))
      (Variables|/Game/Blueprints/Cloud.Cloud_C|SetParticleSpawn _output_get (Variables|Default|GetParticleSpawn))
      (Transformation|AttachComponentToComponent (Variables|/Game/Blueprints/Cloud.Cloud_C|GetDefaultSceneRoot (Variables|Default|GetCloud)) (Variables|Default|GetCloudContainer) "None" "SnapToTarget" "SnapToTarget" "KeepWorld" true)
      ;[1 1 1] Spawn FlashingLight
      (bind _returnvalue_3 (Game|SpawnActorfromClass "/Game/Blueprints/FlashingLight.FlashingLight_C" (Transformation|GetWorldTransform (Variables|Collision|GetCapsuleComponent)) "Undefined" 0 0))
      (bind _output_get_2 (Variables|Default|SetFlashingLight _returnvalue_3))
      (Transformation|AttachComponentToComponent _output_get_2 (Variables|Collision|GetCapsuleComponent) "None" "SnapToTarget" "SnapToTarget" "KeepWorld" true))
    (:then_2
      ;[1 1 1] Setup particle color
      (bind _output_get_3 (Variables|Default|SetColor (Variables|Default|GetParticleColor)))
      (Default|SetParticleColor (Variables|Default|GetCloud) _output_get_3))))

(event Collision|EventActorBeginOverlap
  (params (OtherActor :type Actor%20Object%20Reference))
  (if (Actor|ActorHasTag OtherActor "Damagable")
    (CallFunction|StartDamaging)))

(event Collision|EventActorEndOverlap
  (params (OtherActor :type Actor%20Object%20Reference))
  (if (Actor|ActorHasTag OtherActor "Damagable")
    (CallFunction|StopDamaging)))

(event EventTick
  (params (DeltaSeconds :type Float%20%28single-precision%29))
  (bind _capsulecomponent (Variables|Collision|GetCapsuleComponent))
  (bind _returnvalue (Transformation|GetWorldLocation _capsulecomponent))
  ;[1 1 1] Main update
  (Transformation|SetWorldLocation _capsulecomponent (Math|Vector|MakeVector (.x _returnvalue) 0.0 (.z _returnvalue)) false false)
  (Variables|Default|SetIsFast (>= (Math|Vector|VectorLength (Transformation|GetVelocity)) (Variables|Default|GetFastTreshold)))
  (CallFunction|UpdateReflectionTrajetory)
  (CallFunction|UpdateHealth)
  (CallFunction|UpdateZoom))

(event Input|ActionEvents|InputActionJump
  (params (Key :type Key%20Structure :default "AnyKey"))
  ;[1 1 1] Jump movement
  (:Pressed
    (Character|Jump)))

(event Input|ActionEvents|InputActionParticleDash
  (params (Key :type Key%20Structure :default "AnyKey"))
  (bind _returnvalue (Input|AxisValues|GetMoveRight))
  ;[1 1 1] Particle dash
  (:Pressed
    (Character|LaunchCharacter (Game|GetPlayerCharacter 0) (Math|Vector|MakeVector (* (/ _returnvalue (Math|Float|Absolute(Float) _returnvalue)) (Variables|Default|GetDashSpeed)) 0.0 0.0) true false)
    (CallFunction|PlayDashVibration "/Game/Blueprints/ParticleDashVibration.ParticleDashVibration")
    (Audio|PlaySound2D "/Game/Audio/DashNormal.DashNormal")))

(event Input|ActionEvents|InputActionLightDash
  (params (Key :type Key%20Structure :default "AnyKey"))
  (bind _returnvalue (Input|AxisValues|GetMoveRight))
  (bind _dashspeed (Variables|Default|GetDashSpeed))
  (bind _returnvalue_2 (Math|Float|Absolute(Float) _returnvalue))
  (bind _returnvalue_3 (/ _returnvalue _returnvalue_2))
  (bind _returnvalue_4 (* _returnvalue_3 _dashspeed))
  ;[1 1 1] Decide what type of light dash to take
  (:Pressed
    (if (> (Utilities|Array|Length (Variables|/Game/Blueprints/ReflectionTrajectory.ReflectionTrajectory_C|GetHitLocations (Variables|Default|GetReflectionTrajectory))) 0)
      (Default|FollowTrajectory (Variables|Default|GetFollowTrajetoryMovement) (Variables|Default|GetReflectionTrajectory))
      (else
        ;[1 1 1] Light dash
        (if (!= _returnvalue_4 0.0)
          (CallFunction|PlayDashVibration "/Game/Blueprints/LightDashVibration.LightDashVibration")
          (CallFunction|StartLightMode)
          (Audio|PlaySound2D "/Game/Audio/DashLuz.DashLuz")
          (Character|LaunchCharacter (Math|Vector|MakeVector _returnvalue_4 0.0 0.0) true false)
          (Utilities|FlowControl|Delay 0.4)
          (CallFunction|StopLightMode))))))

(event Input|AxisEvents|InputAxisMoveRight
  (params (AxisValue :type Float%20%28single-precision%29))
  ;[1 1 1] Character movement
  (Pawn|Input|AddMovementInput "1.000000, 0, 0" (* AxisValue (Variables|Default|GetSpeed)) false))

(event Input|KeyboardEvents|LeftBracket
  (params (Key :type Key%20Structure :default "AnyKey"))
  ;[1 1 1] Life debug
  (:Pressed
    (Variables|Default|SetHealth (+ (Variables|Default|GetHealth) 1e+01))
    (Development|PrintString (Utilities|String|ToString(Float) (Variables|Default|GetHealth)))))

(event Input|KeyboardEvents|RightBracket
  (params (Key :type Key%20Structure :default "AnyKey"))
  ;[1 1 1] Life debug
  (:Pressed
    (Variables|Default|SetHealth (+ (Variables|Default|GetHealth) -1e+01))
    (Development|PrintString (Utilities|String|ToString(Float) (Variables|Default|GetHealth)))))

(fn ConstructionScript)